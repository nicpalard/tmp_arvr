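; Pineau target actor that reacts to overlapping Fire, Water and BP_Chair actors with effects and sounds, destroying whichever hits it.
; Fire explodes and ignites it, spawning a looked-after flame and audio, swapping to a sad material and recording the time.
; Water splashes and extinguishes any flame, restoring the happy material, while chairs only trigger sounds.
; Tick destroys the target and its fire effects once it has burned for ten seconds.
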(event OnComponentBeginOverlap(Target)
  (params (OverlappedComponent :type Primitive%20Component%20Object%20Reference) (OtherActor :type Actor%20Object%20Reference) (OtherComp :type Primitive%20Component%20Object%20Reference) (OtherBodyIndex :type Integer) (bFromSweep :type Boolean) (SweepResult :type Hit%20Result%20Structure%20%28by%20ref%29))
  (bind _returnvalue (Utilities|GetClass OtherActor))
  (Utilities|FlowControl|Sequence
    (:then_0
      (Variables|Default|Setimpact (.Location (Collision|BreakHitResult SweepResult))))
    (:then_1
      (Utilities|Casting|CastToFireClass _returnvalue
        (:then
          (Effects|SpawnEmitteratLocation "/Game/Elements/Fire/P_Explosion_Fireball.P_Explosion_Fireball" (Variables|Default|Getimpact))
          (Audio|PlaySoundatLocation "/Game/StarterContent/Audio/Explosion01.Explosion01" (Variables|Default|Getimpact))
          (if (not (Variables|Default|GetisOnFire))
            (bind _returnvalue_2 (Effects|SpawnEmitteratLocation "/Game/StarterContent/Particles/P_Fire.P_Fire" (Variables|Default|Getimpact) "0, 0, 0" "0.500000,0.500000,0.500000"))
            (Variables|Default|SetFire _returnvalue_2)
            (bind _returnvalue_3 (Audio|SpawnSoundatLocation "/Game/StarterContent/Audio/Fire01.Fire01" (Variables|Default|Getimpact) "0, 0, 0" 0.25))
            (Variables|Default|SetFireAudio _returnvalue_3)
            (Variables|Default|SetisOnFire true)
            (Rendering|Material|SetMaterial (Variables|Default|GetTarget) 0 "/Game/LeapSandBox/Target/PineauTarget/M_Sad_Pineau.M_Sad_Pineau")
            (Audio|PlaySoundatLocation "/Game/LeapSandBox/Target/PineauTarget/BM_Pineau_2.BM_Pineau_2" (Variables|Default|Getimpact))
            (Variables|Default|SettimeOnFire (Utilities|Time|GetRealTimeSeconds))))
        (:CastFailed
          (Utilities|Casting|CastToWaterClass _returnvalue
            (:then
              (Effects|SpawnEmitteratLocation "/Game/Elements/Water/P_Water_Splash.P_Water_Splash" (Variables|Default|Getimpact))
              (Audio|SpawnSoundatLocation "/Game/Elements/Water/water_splash.water_splash" (Variables|Default|Getimpact))
              (if (Variables|Default|GetisOnFire)
                (Audio|SpawnSoundatLocation "/Game/Elements/Water/Water_steam.Water_steam" (Variables|Default|Getimpact))
                (Components|DestroyComponent (Variables|Default|GetFire))
                (Audio|Components|Audio|Stop (Variables|Default|GetFireAudio))
                (Components|DestroyComponent (Variables|Default|GetFireAudio))
                (Variables|Default|SetisOnFire false)
                (Rendering|Material|SetMaterial (Variables|Default|GetTarget) 0 "/Game/LeapSandBox/Target/PineauTarget/M_Happy_Pineau.M_Happy_Pineau")
                (Audio|PlaySoundatLocation "/Game/LeapSandBox/Target/PineauTarget/Happy_Pineau.Happy_Pineau" (Variables|Default|Getimpact))))
            (:CastFailed
              (Utilities|Casting|CastToBP_ChairClass _returnvalue)
              (Audio|SpawnSoundatLocation "/Game/LeapSandBox/Target/PineauTarget/BM_Pineau.BM_Pineau" (Variables|Default|Getimpact))
              (Audio|PlaySoundatLocation "/Engine/VREditor/Sounds/UI/Teleport_Committed.Teleport_Committed" (Variables|Default|Getimpact))))))
      (Actor|DestroyActor OtherActor))))

(event EventTick
  (params (DeltaSeconds :type Float%20%28single-precision%29))
  (bind _fireaudio (Variables|Default|GetFireAudio))
  (if (and (>= (- (Utilities|Time|GetRealTimeSeconds) (Variables|Default|GettimeOnFire)) 1e+01) (Variables|Default|GetisOnFire))
    (Actor|DestroyActor)
    (Components|DestroyComponent (Variables|Default|GetFire))
    (Audio|Components|Audio|Stop _fireaudio)
    (Components|DestroyComponent _fireaudio)))

(fn ConstructionScript)